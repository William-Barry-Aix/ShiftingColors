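; BP_DamageBridge1 is a bridge actor whose material reacts to the positions and colours of two player characters.
; BeginPlay creates a dynamic instance of M_DamageBridge_Green on the Bridge mesh.
; Every Tick it finds all BP_DualCharacter actors and feeds the first two's world locations and opposite camera colours into the material's per-player parameters.
; It assumes two characters exist, with no bounds check, and contains no damage logic itself.
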(event EventBeginPlay
  (bind _returnvalue (Rendering|Material|CreateDynamicMaterialInstance (Variables|Default|GetBridge) 0 "/Game/Materials/M_DamageBridge_Green.M_DamageBridge_Green" "None" :!class /Script/Engine.PrimitiveComponent))
  (Variables|Default|SetMatInst _returnvalue))

(event EventTick
  (params (DeltaSeconds :type Float%20%28single-precision%29))
  (bind _outactors (Actor|GetAllActorsOfClass "/Game/ThirdPersonBP/Blueprints/BP_DualCharacter.BP_DualCharacter_C"))
  (Utilities|FlowControl|Sequence
    (:then_0
      (Rendering|Material|SetVectorParameterValue (Variables|Default|GetMatInst) "Pos1" (Math|Conversions|ToLinearColor(Vector) (Transformation|GetWorldLocation (Variables|/Script/Engine.Actor|GetRootComponent (Utilities|Array|Get(acopy) _outactors)))) :!class /Script/Engine.MaterialInstanceDynamic)
      (Rendering|Material|SetVectorParameterValue (Variables|Default|GetMatInst) "ColorPlayer1" (Variables|/Game/ColorShift/CameraColor.CameraColor_C|GetcolorOposite (Variables|/Game/ThirdPersonBP/Blueprints/BP_DualCharacter.BP_DualCharacter_C|GetCameraColor (Utilities|Array|Get(acopy) _outactors))) :!class /Script/Engine.MaterialInstanceDynamic))
    (:then_1
      (Rendering|Material|SetVectorParameterValue (Variables|Default|GetMatInst) "Pos2" (Math|Conversions|ToLinearColor(Vector) (Transformation|GetWorldLocation (Variables|/Script/Engine.Actor|GetRootComponent (Utilities|Array|Get(acopy) _outactors 1)))) :!class /Script/Engine.MaterialInstanceDynamic)
      (Rendering|Material|SetVectorParameterValue (Variables|Default|GetMatInst) "ColorPlayer2" (Variables|/Game/ColorShift/CameraColor.CameraColor_C|GetcolorOposite (Variables|/Game/ThirdPersonBP/Blueprints/BP_DualCharacter.BP_DualCharacter_C|GetCameraColor (Utilities|Array|Get(acopy) _outactors 1))) :!class /Script/Engine.MaterialInstanceDynamic))))

(fn ConstructionScript)