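; Split-screen controller that registers with GM_SpliterScreen and manages switching between full-screen and two-player split-screen play.
; On BeginPlay, if IsDual is set, it creates a second local player and turns on split screen.
; Toggle functions switch the view and whether the first gamepad skips player one.
; NonDualToDual spawns and possesses a BP_DualCharacter for each player, then destroys itself; DualToNonDual is an empty stub.
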(event EventBeginPlay
  ;[1 1 1] Init : 2 Split Screen
  (bind _asgm_spliter_screen (Utilities|Casting|CastToGM_SpliterScreen (Game|GetGameMode)))
  (Variables|/Game/SplitScreener/GM_SpliterScreen.GM_SpliterScreen_C|SetSplitScreenController _asgm_spliter_screen self)
  (if (Variables|Default|GetIsDual)
    (Class|GameplayStatics|CreatePlayer -1)
    (Class|SCSplitScreenController|OnToggleSplitScreen self (not (Variables|Default|GetIsDual)))))

(fn ConstructionScript)

(fn NonDualtoDual
  (bind _self self)
  (bind _returnvalue (Transformation|GetActorTransform _self))
  (Development|PrintString "NonDual to Dual")
  (bind _returnvalue_2 (Game|SpawnActorfromClass "/Game/ThirdPersonBP/Blueprints/BP_DualCharacter.BP_DualCharacter_C" _returnvalue "AlwaysSpawn" 0 0))
  (Pawn|Possess (Game|GetPlayerController 0) _returnvalue_2)
  (bind _returnvalue_3 (Game|SpawnActorfromClass "/Game/ThirdPersonBP/Blueprints/BP_DualCharacter.BP_DualCharacter_C" _returnvalue "AlwaysSpawn" 0 0))
  (Pawn|Possess (Game|GetPlayerController 1) _returnvalue_3)
  (Actor|DestroyActor))

(fn DualtoNonDual)

(fn ToggleFullScreen
  (Class|SCSplitScreenController|OnToggleSplitScreen self true)
  (Class|GameMapsSettings|SetSkipAssigningGamepadtoPlayer1 (Class|GameMapsSettings|GetGameMapsSettings) false))

(fn ToggleSplitScreen
  (Class|SCSplitScreenController|OnToggleSplitScreen self false)
  (Class|GameMapsSettings|SetSkipAssigningGamepadtoPlayer1 (Class|GameMapsSettings|GetGameMapsSettings) true))