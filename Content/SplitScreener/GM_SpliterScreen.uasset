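; Split-screen game mode for a two-player game where two BP_DualCharacters can merge into one BP_NonDualCharacter and split again.
; Tick compares both players' camera colors, storing same and opposite flags with debug prints.
; DualToNonDual spawns the merged pawn between players, possesses it and toggles full screen.
; NonDualToDual spawns two pawns, restores split screen, clears merge toggles and enables RainbowDoor collision.
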(event EventBeginPlay
  ;[1 1 1] Create the second player
  (Class|GameMapsSettings|SetSkipAssigningGamepadtoPlayer1 (Class|GameMapsSettings|GetGameMapsSettings) true))

(event EventTick
  (params (DeltaSeconds :type Float%20%28single-precision%29))
  (bind _asbp_dual_character (Utilities|Casting|CastToBP_DualCharacter (Game|Player|GetPlayerPawn 0)))
  (bind _asbp_dual_character_2 (Utilities|Casting|CastToBP_DualCharacter (Game|Player|GetPlayerPawn 1)))
  (Utilities|FlowControl|Sequence
    (:then_0
      (bind _res (Default|ClosetoColor (Variables|/Game/ThirdPersonBP/Blueprints/BP_DualCharacter.BP_DualCharacter_C|GetCameraColor _asbp_dual_character_2) (Variables|/Game/ColorShift/CameraColor.CameraColor_C|GetcolorMine (Variables|/Game/ThirdPersonBP/Blueprints/BP_DualCharacter.BP_DualCharacter_C|GetCameraColor _asbp_dual_character_2)) (Variables|/Game/ColorShift/CameraColor.CameraColor_C|GetcolorOposite (Variables|/Game/ThirdPersonBP/Blueprints/BP_DualCharacter.BP_DualCharacter_C|GetCameraColor _asbp_dual_character))))
      (bind _output_get (Variables|Default|SetPlayersAreOpositeColors _res))
      (Development|PrintString "Oposite" _output_get true "(R=0.062722,G=1.000000,B=0.000000,A=1.000000)" 0.001))
    (:then_1
      (bind _res_2 (Default|ClosetoColor (Variables|/Game/ThirdPersonBP/Blueprints/BP_DualCharacter.BP_DualCharacter_C|GetCameraColor _asbp_dual_character) (Variables|/Game/ColorShift/CameraColor.CameraColor_C|GetcolorMine (Variables|/Game/ThirdPersonBP/Blueprints/BP_DualCharacter.BP_DualCharacter_C|GetCameraColor _asbp_dual_character_2)) (Variables|/Game/ColorShift/CameraColor.CameraColor_C|GetcolorMine (Variables|/Game/ThirdPersonBP/Blueprints/BP_DualCharacter.BP_DualCharacter_C|GetCameraColor _asbp_dual_character))))
      (bind _output_get_2 (Variables|Default|SetPlayersAreSameColors _res_2))
      (Development|PrintString "Same" _output_get_2 true "(R=0.062722,G=1.000000,B=0.000000,A=1.000000)" 0.001))))

(fn ConstructionScript)

(fn DualtoNonDual
  (params (Playercontroller0 :type Player%20Controller%20Object%20Reference) (Playercontroller1 :type Player%20Controller%20Object%20Reference) (ActorJ0 :type Actor%20Object%20Reference) (ActorJ1 :type Actor%20Object%20Reference))
  (bind _returnvalue (Transformation|GetActorTransform Playercontroller0))
  (bind _returnvalue_2 (Game|SpawnActorfromClass "/Game/ThirdPersonBP/Blueprints/BP_NonDualCharacter.BP_NonDualCharacter_C" (Math|Transform|MakeTransform (/ (+ (.location _returnvalue) (.location (Transformation|GetActorTransform Playercontroller1)) "0,0,10.000000") 2.0) "0, 0, 0" (.scale _returnvalue)) "AlwaysSpawn" 0 0))
  (Pawn|Possess Playercontroller1 _returnvalue_2)
  (Pawn|Possess Playercontroller0 _returnvalue_2)
  (Actor|DestroyActor ActorJ1)
  (Actor|DestroyActor ActorJ0)
  (Default|ToggleFullScreen (Variables|Default|GetSplitScreenController)))

(fn NonDualtoDual
  (params (Playercontroller0 :type Player%20Controller%20Object%20Reference) (Playercontroller1 :type Player%20Controller%20Object%20Reference) (Player0 :type Actor%20Object%20Reference))
  (bind _returnvalue (Transformation|GetActorTransform Playercontroller0))
  (Utilities|FlowControl|Sequence
    (:then_0
      (bind _returnvalue_2 (Game|SpawnActorfromClass "/Game/ThirdPersonBP/Blueprints/BP_DualCharacter.BP_DualCharacter_C" (Math|Transform|MakeTransform (+ (.location _returnvalue) "2.000000, 0, 0")) "Undefined" 0 0))
      (Pawn|Possess Playercontroller0 _returnvalue_2))
    (:then_1
      (bind _returnvalue_3 (Game|SpawnActorfromClass "/Game/ThirdPersonBP/Blueprints/BP_DualCharacter.BP_DualCharacter_C" (Math|Transform|MakeTransform (+ (.location _returnvalue) "-2.000000, 0, 0")) "Undefined" 0 0))
      (Pawn|Possess Playercontroller1 _returnvalue_3))
    (:then_2
      (Actor|DestroyActor Player0)
      (Default|ToggleSplitScreen (Variables|Default|GetSplitScreenController)))
    (:then_3
      (Variables|Default|SetJ1ToggleMerge false)
      (Variables|Default|SetJ0ToggleMerge false))
    (:then_4
      (Default|SetonCollide (Variables|Default|GetRainbowDoor) true))))